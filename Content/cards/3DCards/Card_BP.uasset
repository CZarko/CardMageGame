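; Collectible 3D card actor that vanishes when a BP_MageCharacter overlaps it and respawns after a 30-second delay.
; On BeginPlay and each respawn it randomly takes a Pyro, Cryo or Electro Blast card material.
; Overlap disables the mesh's visibility, collision and tick, adds one of two random audio components and records the time.
; Tick polls that timestamp to re-enable the card; no ability is granted here.
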(event EventBeginPlay
  (bind _card (Variables|Default|GetCard))
  (switch int (Math|Random|RandomIntegerinRange 0 2)
    (:0
      (|CollapseGraph _card _card _card :!label _label))
    (:1
      (goto _label execute2))
    (:2
      (goto _label execute3))))

(event Collision|EventActorBeginOverlap
  (params (OtherActor :type Actor%20Object%20Reference))
  (Utilities|Casting|CastToBP_MageCharacter OtherActor)
  (CallFunction|DisableCard)
  (switch int (Math|Random|RandomIntegerinRange 0 1)
    (:0
      (AddComponent|AddAudioComponent false))
    (:1
      (AddComponent|AddAudioComponent false)))
  (bind _output_get (Variables|Components|SetDestroyedTime (Utilities|Time|GetTimeSeconds))))

(event EventTick
  (params (DeltaSeconds :type Float%20%28single-precision%29))
  (bind _card (Variables|Default|GetCard))
  (if (and (> (Utilities|Time|GetTimeSeconds) (+ 3e+01 (stale Collision|EventActorBeginOverlap _output_get))) (!= (Variables|Components|GetDestroyedTime) 0.0))
    (Variables|Components|SetDestroyedTime 0.0)
    (CallFunction|EnableCard)
    (switch int (Math|Random|RandomIntegerinRange 0 2)
      (:0
        (|CollapseGraph _card _card _card :!label _label))
      (:1
        (goto _label execute2))
      (:2
        (goto _label execute3)))))

(fn ConstructionScript)

(fn DisableCard
  (bind _card (Variables|Default|GetCard))
  (Components|Activation|Deactivate _card)
  (Rendering|SetVisibility _card false false)
  (Collision|SetCollisionEnabled _card "NoCollision")
  (Components|Tick|SetComponentTickEnabled _card false))

(fn EnableCard
  (bind _card (Variables|Default|GetCard))
  (Components|Activation|Deactivate _card)
  (Rendering|SetVisibility _card true false)
  (Collision|SetCollisionEnabled _card "QueryAndPhysics")
  (Components|Tick|SetComponentTickEnabled _card true))